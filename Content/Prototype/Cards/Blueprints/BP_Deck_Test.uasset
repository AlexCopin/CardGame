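; BP_Deck_Test is a prototype deck actor that spawns a row of BP_Card actors when play begins.
; CreateDeck looks up each entry in CardIds in the CardList data table held by the CG_GameStateBase game state.
; Each found row spawns a card stepped by Offset from the deck's transform, sets its plane material to the card image, initializes it and stores it in Cards.
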(event EventBeginPlay
  (CallFunction|CreateDeck))

(event Collision|EventActorBeginOverlap
  (params (OtherActor :type Actor%20Object%20Reference)))

(event EventTick
  (params (DeltaSeconds :type Float%20%28single-precision%29)))

(fn ConstructionScript)

(fn CreateDeck
  (bind _returnvalue (Transformation|GetActorTransform))
  (bind _ascg_game_state_base (Utilities|Casting|CastToCG_GameStateBase (Game|GetGameState)))
  (for (_array_element _array_index) (Variables|Default|GetCardIds)
    (bind _returnvalue_2 (Utilities|GetDataTableRow (Variables|/Script/CardGame.CG_GameStateBase|GetCardList _ascg_game_state_base) _array_element)
      (:then
        (bind _structout (Utilities|Struct|SetmembersinCardData _returnvalue_2))
        (bind _returnvalue_3 (Game|SpawnActorfromClass "/Game/Prototype/Cards/Blueprints/BP_Card.BP_Card_C" (Math|Transform|MakeTransform (+ (.location _returnvalue) (* (LocalVariables|GetOffset) _array_index)) (.rotation _returnvalue) (.scale _returnvalue)) "Undefined" "MultiplyWithRoot" (Components|GetOwner) 0))
        (Rendering|Material|SetMaterial (Variables|/Game/Prototype/Cards/Blueprints/BP_Card.BP_Card_C|GetPlane _returnvalue_3) 0 (Utilities|Struct|BreakCardData _structout))
        (Class|Card|Init _returnvalue_3 _structout)
        (Utilities|Array|Add (Variables|Default|GetCards) _returnvalue_3)))))