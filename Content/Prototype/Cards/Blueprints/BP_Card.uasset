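; Prototype card actor that shows its CardData image on a plane and displays Health and Attack through stat widgets.
; SetStyle extends the parent styling, applies the image material and starts timers.
; A looping timer retries binding both WBP_CardStat widgets to the card, clearing itself once the Attack binding succeeds.
; Delayed test events change Health through ServerAddToStats, apparently to exercise stat updates.
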(event Custom|AddToStatTest
  (Class|Card|ServerAddtoStats "(TagName=\"Stat.Card.Health\")" -2))

(event Custom|AddToStatTest2
  (Class|Card|ServerAddtoStats "(TagName=\"Stat.Card.Health\")" 3))

(event Custom|UpdateStartToBind
  (bind _aswbp_card_stat (Utilities|Casting|CastToWBP_CardStat (UserInterface|GetUserWidgetObject (Variables|Default|GetHealthWidget))))
  (Default|SetCard _aswbp_card_stat self "(TagName=\"Stat.Card.Health\")")
  (bind _aswbp_card_stat_2 (Utilities|Casting|CastToWBP_CardStat (UserInterface|GetUserWidgetObject (Variables|Default|GetAttackWidget))))
  (bind _success (Default|SetCard _aswbp_card_stat_2 self "(TagName=\"Stat.Card.Attack\")"))
  (if _success
    (Development|PrintString "Bind successful")
    (Utilities|Time|ClearandInvalidateTimerbyHandle (Variables|Default|GetTimer))
    (else
      (Development|PrintString "BP Card failed to bind to widgets"))))

(event EventSetStyle
  (|CallParentFunction)
  (Rendering|Material|SetMaterial (Variables|Default|GetPlane) 0 (Utilities|Struct|BreakCardData (Variables|Default|GetCardData)))
  (bind _returnvalue (Utilities|Time|SetTimerbyEvent (EventDispatchers|CreateEvent :!event Custom|UpdateStartToBind) 0.3 true))
  (Variables|Default|SetTimer _returnvalue)
  (bind _returnvalue_2 (Utilities|Time|SetTimerbyEvent (EventDispatchers|CreateEvent :!event Custom|AddToStatTest) 5.0))
  (Variables|Default|SetTimerStatTest _returnvalue_2)
  (Utilities|Time|SetTimerbyEvent (EventDispatchers|CreateEvent :!event Custom|AddToStatTest2) 1e+01))

(fn ConstructionScript)